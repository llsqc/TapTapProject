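; BP_PickableItem is a world pickup that adds an item to the player's inventory on contact.
; On BeginPlay it applies its configured flipbook to the Paper2D flipbook component.
; When the player character overlaps its sphere, it casts to BP_Aura, passes its ItemID and Quantity to that character's InventoryComponent, then destroys itself.
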(event `self.ReceiveBeginPlay`
  (`PaperFlipbookComponent.SetFlipbook` (`self.PaperFlipbook`) (`self.New Flipbook`)))

(event `self.Sphere.OnComponentBeginOverlap`
  (params (OverlappedComponent :type "PrimitiveComponent Object Reference") (OtherActor :type "Actor Object Reference") (OtherComp :type "PrimitiveComponent Object Reference") (OtherBodyIndex :type Integer) (bFromSweep :type Boolean) (SweepResult :type "HitResult Structure (by ref)"))
  (if (== OtherActor (`GameplayStatics.GetPlayerCharacter` 0))
    (bind _asbp_aura (cast `/Game/_Game/Character/Aura/BP_Aura` OtherActor))
    (`/Game/_Game/Character/Aura/Inventory/InventoryComponent.AddToInventory` (`/Game/_Game/Character/Aura/BP_Aura.InventoryComponent` _asbp_aura) (`self.ItemID`) (`self.Quantity`))
    (`self.K2_DestroyActor`)))

(fn `UserConstructionScript`)
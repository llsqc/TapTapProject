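; BP_Shopkeeper is a world shopkeeper actor that opens a shop UI for the player.
; Its ShopTrigger overlap sets OverlapShop on the player's BP_Aura and binds an open-shop callback; leaving clears the flag without unbinding.
; The callback ignores move input, blends the view to the shopkeeper, then after a short delay shows WBP_Shopkeeper with a self reference and switches to UI-only input.
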(event `self.ShopTrigger.OnComponentBeginOverlap`
  (params (OverlappedComponent :type "PrimitiveComponent Object Reference") (OtherActor :type "Actor Object Reference") (OtherComp :type "PrimitiveComponent Object Reference") (OtherBodyIndex :type Integer) (bFromSweep :type Boolean) (SweepResult :type "HitResult Structure (by ref)"))
  (bind _returnvalue (`GameplayStatics.GetPlayerCharacter` 0))
  (if (== OtherActor _returnvalue)
    (bind _asbp_aura (cast `/Game/_Game/Character/Aura/BP_Aura` _returnvalue))
    (set `/Game/_Game/Character/Aura/BP_Aura.bOverlapShop` true _asbp_aura)
    (add `/Game/_Game/Character/Aura/BP_Aura.OpenTheShop` _asbp_aura (delegate `自定义事件`))))

(event `自定义事件`
  (bind _returnvalue (`GameplayStatics.GetPlayerController` 0))
  (`Controller.SetIgnoreMoveInput` _returnvalue true)
  (`PlayerController.SetViewTargetWithBlend` _returnvalue self 0.5 "VTBlend_Linear" 0.0 false)
  (`KismetSystemLibrary.Delay` 0.5)
  (bind _returnvalue_2 (`|CreateWidget` "/Game/_Game/WorldObject/Shop/WBP_Shopkeeper.WBP_Shopkeeper_C" null self))
  (`UserWidget.AddToViewport` _returnvalue_2 0)
  (`WidgetBlueprintLibrary.SetInputMode_UIOnlyEx` (`GameplayStatics.GetPlayerController` 0) null))

(event `self.ShopTrigger.OnComponentEndOverlap`
  (params (OverlappedComponent :type "PrimitiveComponent Object Reference") (OtherActor :type "Actor Object Reference") (OtherComp :type "PrimitiveComponent Object Reference") (OtherBodyIndex :type Integer))
  (bind _returnvalue (`GameplayStatics.GetPlayerCharacter` 0))
  (if (== OtherActor _returnvalue)
    (bind _asbp_aura (cast `/Game/_Game/Character/Aura/BP_Aura` _returnvalue))
    (set `/Game/_Game/Character/Aura/BP_Aura.bOverlapShop` false _asbp_aura)))

(fn `UserConstructionScript`)
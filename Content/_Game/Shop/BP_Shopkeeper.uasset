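; BP_Shopkeeper is the shopkeeper actor that opens the shop UI when the player character enters its ShopTrigger.
; On overlap it blends the player's view to itself, then after a short delay creates WBP_Shopkeeper with a reference back to this actor.
; It adds the widget to the viewport and switches input to UI-only; closing the shop is not handled in this graph.
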(event `self.ShopTrigger.OnComponentBeginOverlap`
  (params (OverlappedComponent :type "PrimitiveComponent Object Reference") (OtherActor :type "Actor Object Reference") (OtherComp :type "PrimitiveComponent Object Reference") (OtherBodyIndex :type Integer) (bFromSweep :type Boolean) (SweepResult :type "HitResult Structure (by ref)"))
  (if (== OtherActor (`GameplayStatics.GetPlayerCharacter` 0))
    (`PlayerController.SetViewTargetWithBlend` (`GameplayStatics.GetPlayerController` 0) self 0.5 "VTBlend_Linear" 0.0 false)
    (`KismetSystemLibrary.Delay` 0.2)
    (bind _returnvalue (`|CreateWidget` "/Game/_Game/Shop/WBP_Shopkeeper.WBP_Shopkeeper_C" null self))
    (`UserWidget.AddToViewport` _returnvalue 0)
    (`WidgetBlueprintLibrary.SetInputMode_UIOnlyEx` (`GameplayStatics.GetPlayerController` 0) null "LockOnCapture")))

(fn `UserConstructionScript`)
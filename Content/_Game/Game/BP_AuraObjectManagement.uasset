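; BP_AuraObjectManagement is a manager actor that pools BP_Projectile actors for reuse.
; On BeginPlay it registers itself as ObjectManagement on the Aura game instance.
; SetProjectilePool takes the first pooled projectile in the reusable state, or spawns one at a far-off location and adds it to the pool.
; It then initializes that projectile with the supplied flipbook, combat stats, target tag and life cycle, and moves it to the requested location.
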(event `self.ReceiveBeginPlay`
  (set `/Game/_Game/Game/BP_AuraGameInstance.ObjectManagement` self (`/Game/_Game/Game/BP_BluePrintLibrary.GetAuraGameInstance`)))

(fn `SetProjectilePool`
  (params (ProjectileLocation :type "Vector Structure") (ProjectileFlipbook :type "PaperFlipbook Object Reference") (ProjectileDamage :type "Float (double-precision)") (ProjectileSpeed :type "Vector Structure") (ProjectileSize :type "Vector Structure") (ProjectileHitRange :type "Vector Structure") (TagOfHitActor :type Name) (LifeCycle :type "Float (double-precision)"))
  (locals (Projectile :type "/Game/_Game/Character/Weapon/Projectile/BP_Projectile Object Reference"))
  (bind _projectile (`local.Projectile`))
  (for _array_element (`self.ProjectilePool`)
    (if (`|EnumEquality` (`/Game/_Game/Character/Weapon/Projectile/BP_Projectile.ProjectileState` _array_element) "NewEnumerator1")
      (set `local.Projectile` _array_element)
      (break)))
  (`local.Projectile`
    (:`then`
      _)
    (:`else`
      (bind _returnvalue (`|SpawnActorFromClass` "/Game/_Game/Character/Weapon/Projectile/BP_Projectile.BP_Projectile_C" (`KismetMathLibrary.MakeTransform` (10000.0 10000.0 10000.0)) "Undefined" "MultiplyWithRoot" null null))
      (bind _output_get (set `local.Projectile` _returnvalue))
      (`KismetArrayLibrary.Array_Add` (`self.ProjectilePool`) _output_get)))
  (`/Game/_Game/Character/Weapon/Projectile/BP_Projectile.InitializeProjectile` _projectile (`local.ProjectileFlipbook`) (`local.ProjectileDamage`) (`local.ProjectileSpeed`) (`local.ProjectileSize`) (`local.ProjectileHitRange`) (`local.TagOfHitActor`) (`local.LifeCycle`))
  (`self.K2_SetActorLocation` _projectile (`local.ProjectileLocation`) false false))

(fn `UserConstructionScript`)
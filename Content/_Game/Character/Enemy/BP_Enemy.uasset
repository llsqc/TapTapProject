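; BP_Enemy is a sprite-based enemy character that chases the player, configured by EnemyDataAsset for walk speed and animation.
; Pursuit uses AIMoveTo, restarting on success and starting a looping timer on failure.
; Tick forces zero rotation to keep the actor's orientation fixed.
; UnderAttack flashes the sprite red, plays a sound, then shows damage through a lazily spawned, reused BP_DamageNumber attached to the sprite.
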(event `self.ReceiveBeginPlay`
  (bind _enemydataasset (`self.EnemyDataAsset`))
  (bind _asabp_enemy (cast `/Game/_Game/Character/Enemy/ABP_Enemy` (`self.GetAnimInstance`)))
  (bind _output_get (set `self.As ABP Enemy` _asabp_enemy))
  (set `/Game/_Game/Character/Enemy/ABP_Enemy.Anim Sequence` (`self.Anim Sequence`) _output_get)
  (set `self.Anim Sequence` (`/Game/_Game/DataAsset/BP_EnemyDataAsset.EnemyAnim` _enemydataasset))
  (set `CharacterMovementComponent.MaxWalkSpeed` (`/Game/_Game/DataAsset/BP_EnemyDataAsset.EnemySpeed` _enemydataasset) (`self.CharacterMovement`))
  (`self.StartPursue`))

(event `StartPursue`
  (bind _returnvalue (`GameplayStatics.GetPlayerPawn` 0))
  (`KismetSystemLibrary.Delay` 0.2)
  (`/Engine/EditorBlueprintResources/StandardMacros.IsValid` _returnvalue
    (:`Is Valid`
      (`|AIMoveTo` self (0.0 0.0 0.0) _returnvalue
        (:`OnSuccess`
          (`KismetSystemLibrary.K2_ClearAndInvalidateTimerHandle` (`self.PursueTimerHandle`))
          (`self.StartPursue`))
        (:`OnFail`
          (bind _returnvalue_2 (`KismetSystemLibrary.K2_SetTimerDelegate` (`|CreateDelegate` :!event `StartPursue`) 0.5 true))
          (set `self.PursueTimerHandle` _returnvalue_2))))))

(event `self.ReceiveTick`
  (params (DeltaSeconds :type "Float (single-precision)"))
  (`self.K2_SetActorRotation` (struct)))

(event `/Game/_Game/Interface/BP_CombatInterface.UnderAttack`
  (params (Damage :type "Float (double-precision)"))
  (`PaperFlipbookComponent.SetSpriteColor` (`self.Sprite`) (struct :`R` 1.0 :`A` 1.0))
  (`GameplayStatics.PlaySound2D` "/Game/_Game/Sound/SoundEffect/Cue_DamageSound.Cue_DamageSound" 1.0 1.0 0.0 null null)
  (`KismetSystemLibrary.Delay` 0.2)
  (`self.ShowDamage` (`KismetTextLibrary.Conv_IntToText` (`KismetMathLibrary.FTrunc` Damage)))
  (`PaperFlipbookComponent.SetSpriteColor` (`self.Sprite`) (struct :`R` 1.0 :`G` 1.0 :`B` 1.0 :`A` 1.0)))

(fn `ShowDamage`
  (params (DamageNumber :type Text))
  (`self.DamageNumberContianer`
    (:`then`
      _)
    (:`else`
      (bind _returnvalue (`|SpawnActorFromClass` "/Game/_Game/UI/BP_DamageNumber.BP_DamageNumber_C" (`KismetMathLibrary.MakeTransform` (`SceneComponent.K2_GetComponentLocation` (`self.Sprite`))) "AlwaysSpawn" "MultiplyWithRoot" null null))
      (bind _output_get (set `self.DamageNumberContianer` _returnvalue))
      (`self.K2_AttachToComponent` _output_get (`self.Sprite`) "None" "KeepWorld" "KeepWorld" "KeepWorld" true)))
  (`/Game/_Game/UI/BP_DamageNumber.ShowDamageNumber` (`self.DamageNumberContianer`) DamageNumber))

(fn `UserConstructionScript`)
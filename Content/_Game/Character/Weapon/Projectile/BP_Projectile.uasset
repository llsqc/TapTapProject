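; BP_Projectile is a Paper2D flipbook projectile that its spawner configures at runtime.
; InitializeProjectile sets the flipbook and its scale, the movement velocity and the sphere's hit-range scale, and stores damage and a target actor tag.
; It also starts a lifetime timer by function name that calls RecycleProjectile, which destroys the actor rather than pooling it.
; The event graph is inactive, so no overlap or damage handling happens here.
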(fn `InitializeProjectile`
  (params (ProjectileFlipbook :type "PaperFlipbook Object Reference") (ProjectileDamage :type "Float (double-precision)") (ProjectileSpeed :type "Vector Structure") (ProjectileSize :type "Vector Structure") (ProjectileHitRange :type "Vector Structure") (TagOfHitActor :type Name) (LifeCycle :type "Float (double-precision)"))
  (`PaperFlipbookComponent.SetFlipbook` (`self.PaperFlipbook`) ProjectileFlipbook)
  (set `self.Projectile Damage` ProjectileDamage)
  (set `MovementComponent.Velocity` ProjectileSpeed (`self.ProjectileMovement`))
  (`SceneComponent.SetWorldScale3D` (`self.PaperFlipbook`) ProjectileSize)
  (`SceneComponent.SetWorldScale3D` (`self.Sphere`) ProjectileHitRange)
  (set `self.Tag Of Hit Actor` TagOfHitActor)
  (`KismetSystemLibrary.K2_SetTimer` null "RecycleProjectile" LifeCycle))

(fn `RecycleProjectile`
  (`self.K2_DestroyActor`))

(fn `UserConstructionScript`)
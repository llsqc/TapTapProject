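; BP_Aura is the player character, which registers itself with the Aura game instance on BeginPlay.
; Enhanced Input moves it along world X/Y and opens the inventory widget in UI-only input mode.
; Shooting aims by yaw at the cursor hit point and requests an enemy-damaging fireball from the game instance's projectile pool.
; A SpendMoney function updates and returns Money.
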(event `self.ReceiveBeginPlay`
  (bind _bp_auragameinstance (`/Game/_Game/Game/BP_BluePrintLibrary.GetAuraGameInstance`))
  (set `/Game/_Game/Game/BP_AuraGameInstance.Aura` self _bp_auragameinstance)
  (set `self.BP Aura Game Instance` _bp_auragameinstance))

(event `EnhancedInput|/Game/_Game/Input/IA_Move`
  (params (ActionValue :type "Vector2D Structure") (ElapsedSeconds :type "Float (double-precision)") (TriggeredSeconds :type "Float (double-precision)") (InputAction :type "InputAction Object Reference" :default "/Game/_Game/Input/IA_Move.IA_Move"))
  (bind (_x _y) (`KismetMathLibrary.BreakVector2D` ActionValue))
  (:`Triggered`
    (set `self.X` _x)
    (set `self.Y` _y)
    (`self.AddMovementInput` (1.0 0.0 0.0) _x)
    (`self.AddMovementInput` (0.0 1.0 0.0) _y)))

(event `EnhancedInput|/Game/_Game/Input/IA_Shoot`
  (params (ActionValue :type Boolean) (ElapsedSeconds :type "Float (double-precision)") (TriggeredSeconds :type "Float (double-precision)") (InputAction :type "InputAction Object Reference" :default "/Game/_Game/Input/IA_Shoot.IA_Shoot"))
  (bind (_returnvalue_roll _returnvalue_pitch _returnvalue_yaw) (`KismetMathLibrary.BreakRotator` (`KismetMathLibrary.FindLookAtRotation` (`self.K2_GetActorLocation`) (`.Location` (`GameplayStatics.BreakHitResult` (`PlayerController.GetHitResultUnderCursorByChannel` (`GameplayStatics.GetPlayerController` 0) "TraceTypeQuery1" true))))))
  (:`Started`
    (`/Game/_Game/Game/BP_AuraObjectManagement.SetProjectilePool` (`/Game/_Game/Game/BP_AuraGameInstance.ObjectManagement` (`self.BP Aura Game Instance`)) (`self.K2_GetActorLocation`) "/Game/_Game/Character/Weapon/Projectile/FireBall/Fire_ball.Fire_ball" 5.0 (* (`KismetMathLibrary.Conv_RotatorToVector` (`KismetMathLibrary.MakeRotator` 0.0 0.0 _returnvalue_yaw)) 400) (1.0 1.0 1.0) (1.0 1.0 1.0) "Enemy" 1.0)))

(event `EnhancedInput|/Game/_Game/Input/IA_Inventory`
  (params (ActionValue :type Boolean) (ElapsedSeconds :type "Float (double-precision)") (TriggeredSeconds :type "Float (double-precision)") (InputAction :type "InputAction Object Reference" :default "/Game/_Game/Input/IA_Inventory.IA_Inventory"))
  (:`Started`
    (bind _returnvalue (`|CreateWidget` "/Game/_Game/Shop/WBP_PlayerInventory.WBP_PlayerInventory_C" null null))
    (`UserWidget.AddToViewport` _returnvalue 0)
    (`WidgetBlueprintLibrary.SetInputMode_UIOnlyEx` (`GameplayStatics.GetPlayerController` 0) null)))

(fn `SpendMoney`
  (params (Money :type Integer))
  (returns (RemainingMoney :type Integer))
  (bind _output_get (set `self.Money` (- (`self.Money`) Money)))
  (return _output_get))

(fn `UserConstructionScript`)